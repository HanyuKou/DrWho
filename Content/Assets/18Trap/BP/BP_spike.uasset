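; Paper2D flipbook spike trap that respawns Pawn_DrWho_Lab on contact.
; Trigger toggles the spikes, either externally or via a BeginPlay loop with on/off delays, playing the flipbook alongside a rate-matched timeline that resizes the Box collision.
; Overlap respawns the pawn immediately when spikes are up, otherwise polls each tick until the animation passes a threshold.
; The construction script poses the initial up or down state.
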(event `self.ReceiveBeginPlay`
  (if (not (and (== (`self.triggerLoopOn`) 0.0) (== (`self.triggerLoopOff`) 0.0)))
    (`self.LoopSpike`)))

(event `LoopSpike`
  (`self.Trigger` false :!label _label)
  (if (`self.SpikeOn`)
    (`KismetSystemLibrary.Delay` (`self.triggerLoopOn`))
    (goto _label)
    (else
      (`KismetSystemLibrary.Delay` (`self.triggerLoopOff`))
      (goto _label))))

(event `StopSpike`
  (bind _spikeon (`self.SpikeOn`))
  (bind _rendercomponent (`self.RenderComponent`))
  (bind (_direction _newtrack_0) (`Timeline|SpikeUp` :!via `Stop` :!label _label_2)
    (:`Update`
      (set `self.timelineAlpha` _newtrack_0)
      (`BoxComponent.SetBoxExtent` (`self.Box`) (`KismetMathLibrary.VLerp` (14.5 16.0 0.0) (14.5 16.0 6.0) _newtrack_0) true))
    (:`Finished`
      (set `self.SpikeOn` (not _spikeon))
      (if (stale `Trigger` loop)
        (if _spikeon :!label _label_3
          (`PaperFlipbookComponent.ReverseFromEnd` _rendercomponent)
          (goto _label_2 :!via `ReverseFromEnd`)
          (else
            (`PaperFlipbookComponent.Play` _rendercomponent)
            (goto _label_2 :!via `PlayFromStart`)))))))

(event `Trigger`
  (params (loop :type Boolean))
  (`TimelineComponent.SetPlayRate` (`self.SpikeUp`) (/ 1.0 (`PaperFlipbookComponent.GetFlipbookLength` (`self.RenderComponent`))))
  (goto _label_3))

(event `self.Box_overlap.OnComponentBeginOverlap`
  (params (OverlappedComponent :type "PrimitiveComponent Object Reference") (OtherActor :type "Actor Object Reference") (OtherComp :type "PrimitiveComponent Object Reference") (OtherBodyIndex :type Integer) (bFromSweep :type Boolean) (SweepResult :type "HitResult Structure (by ref)"))
  (bind _rendercomponent (`self.RenderComponent`))
  (if (`self.SpikeOn`)
    (bind _aspawn_dr_who_lab (cast `/Game/Assets/puzzle_platformer_kit/BP/Pawn_DrWho_Lab` OtherActor))
    (`/Engine/EditorBlueprintResources/StandardMacros.DoOnce` false
      (:`Completed`
        (`/Game/Assets/puzzle_platformer_kit/BP/Pawn_DrWho_Lab.Respawn` _aspawn_dr_who_lab)))
    (else
      (if (== (`KismetArrayLibrary.Array_Length` (`PrimitiveComponent.GetOverlappingActors` (`self.Box_overlap`) "/Game/Assets/puzzle_platformer_kit/BP/Pawn_DrWho_Lab.Pawn_DrWho_Lab_C")) 0) :!label _label_4
        _
        (elif (> (`PaperFlipbookComponent.GetPlaybackPosition` _rendercomponent) (* (`PaperFlipbookComponent.GetFlipbookLength` _rendercomponent) 0.45))
          (`/Engine/EditorBlueprintResources/StandardMacros.DoOnce` false
            (:`Completed`
              (bind _aspawn_dr_who_lab_2 (cast `/Game/Assets/puzzle_platformer_kit/BP/Pawn_DrWho_Lab` (`GameplayStatics.GetPlayerPawn` 0)))
              (`/Game/Assets/puzzle_platformer_kit/BP/Pawn_DrWho_Lab.Respawn` _aspawn_dr_who_lab_2)))
          (else
            (`KismetSystemLibrary.DelayUntilNextTick`)
            (goto _label_4)))))))

(fn `UserConstructionScript`
  (bind _rendercomponent (`self.RenderComponent`))
  (`PaperFlipbookComponent.Stop` _rendercomponent)
  (if (`self.SpikeOn`)
    (`PaperFlipbookComponent.SetPlaybackPosition` _rendercomponent (`PaperFlipbookComponent.GetFlipbookLength` _rendercomponent) false)
    (`BoxComponent.SetBoxExtent` (`self.Box`) (14.5 16.0 6.0) true)
    (else
      (`PaperFlipbookComponent.SetPlaybackPosition` _rendercomponent 0.0 false)))
  (`PaperFlipbookComponent.SetLooping` _rendercomponent false))