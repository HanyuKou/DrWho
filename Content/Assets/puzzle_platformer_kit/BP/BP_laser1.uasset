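; A laser hazard for a puzzle platformer that respawns the Pawn_DrWho_Lab player when it overlaps the Box while the laser is on.
; Trigger toggles LaserOn along with the render component's visibility and collision.
; Unless both loop timers are zero, BeginPlay starts LoopLaser, an endless Delay loop that waits TriggerLoopOff while on or TriggerLoopOn while off, then calls Trigger.
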(event `self.ReceiveBeginPlay`
  (if (not (and (== (`self.triggerLoopOn`) 0.0) (== (`self.triggerLoopOff`) 0.0)))
    (`self.LoopLaser`)))

(event `BoxOverlapEvent`
  (params (actorObj :type "Actor Object Reference"))
  (if (`self.LaserOn`)
    (bind _aspawn_dr_who_lab (cast `/Game/Assets/puzzle_platformer_kit/BP/Pawn_DrWho_Lab` actorObj))
    (`/Game/Assets/puzzle_platformer_kit/BP/Pawn_DrWho_Lab.Respawn` _aspawn_dr_who_lab)))

(event `self.Box.OnComponentBeginOverlap`
  (params (OverlappedComponent :type "PrimitiveComponent Object Reference") (OtherActor :type "Actor Object Reference") (OtherComp :type "PrimitiveComponent Object Reference") (OtherBodyIndex :type Integer) (bFromSweep :type Boolean) (SweepResult :type "HitResult Structure (by ref)"))
  (`self.BoxOverlapEvent` OtherActor))

(event `LoopLaser`
  (if (`self.LaserOn`) :!label _label
    (`KismetSystemLibrary.Delay` (`self.triggerLoopOff`))
    (else
      (`KismetSystemLibrary.Delay` (`self.triggerLoopOn`))))
  (`self.Trigger`)
  (goto _label))

(event `Trigger`
  (bind _rendercomponent (`self.RenderComponent`))
  (bind _rendercomponent_2 (`self.RenderComponent`))
  (if (`self.LaserOn`)
    (set `self.LaserOn` false)
    (`SceneComponent.SetVisibility` _rendercomponent_2 false false)
    (`PrimitiveComponent.SetCollisionEnabled` _rendercomponent "NoCollision")
    (else
      (set `self.LaserOn` true)
      (`SceneComponent.SetVisibility` _rendercomponent_2 true false)
      (`PrimitiveComponent.SetCollisionEnabled` _rendercomponent "QueryAndPhysics"))))

(fn `UserConstructionScript`)