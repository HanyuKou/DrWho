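; Pressure-plate button for a puzzle platformer that triggers its connected objects while the player pawn (Pawn_DrWho_Lab) or a BP_cube rests on it.
; On box overlap it swaps to the pressed sprite and calls TriggerConnected, then polls the overlap count every tick until empty.
; Once empty, it restores the sprite and triggers the connections with CloseConnected set.
; It overrides the parent's TempTrigger with nothing.
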(event `self.ReceiveBeginPlay`
  (`parent.ReceiveBeginPlay`))

(event `self.BoxOverlapEvent`
  (bind _box (`self.Box`))
  (bind _box_2 (`self.Box`))
  (if (== (+ (`KismetArrayLibrary.Array_Length` (`PrimitiveComponent.GetOverlappingActors` _box "/Game/Assets/puzzle_platformer_kit/BP/Pawn_DrWho_Lab.Pawn_DrWho_Lab_C")) (`KismetArrayLibrary.Array_Length` (`PrimitiveComponent.GetOverlappingActors` _box "/Game/Assets/puzzle_platformer_kit/BP/BP_cube.BP_cube_C"))) 0) :!label _label
    _
    (elif (`self.ButtonOn`)
      (set `self.ButtonOn` false)
      (`PaperSpriteComponent.SetSprite` (`self.RenderComponent`) "/Game/Assets/puzzle_platformer_kit/Sprite/button2_2.button2_2")
      (`self.TriggerConnected` false true)
      (set `self.Ready` true)
      (if (== (+ (`KismetArrayLibrary.Array_Length` (`PrimitiveComponent.GetOverlappingActors` _box_2 "/Game/Assets/puzzle_platformer_kit/BP/Pawn_DrWho_Lab.Pawn_DrWho_Lab_C")) (`KismetArrayLibrary.Array_Length` (`PrimitiveComponent.GetOverlappingActors` _box_2 "/Game/Assets/puzzle_platformer_kit/BP/BP_cube.BP_cube_C"))) 0) :!label _label_2
        (set `self.ButtonOn` true)
        (`PaperSpriteComponent.SetSprite` (`self.RenderComponent`) "/Game/Assets/puzzle_platformer_kit/Sprite/button2_1.button2_1")
        (`self.TriggerConnected` true)
        (set `self.Ready` true)
        (else
          (`KismetSystemLibrary.DelayUntilNextTick`)
          (goto _label_2)))
      (else
        (`KismetSystemLibrary.DelayUntilNextTick`)
        (goto _label)))))

(event `self.tempTrigger`)

(fn `UserConstructionScript`
  (`parent.UserConstructionScript`))