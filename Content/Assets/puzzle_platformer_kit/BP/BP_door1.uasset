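; BP_door1 is a flipbook-animated door that toggles between on and off states in a puzzle platformer.
; Construction stops the non-looping flipbook on its first frame, and Trigger plays it forward or from the end backward, reversing it if already mid-animation.
; When playback finishes, the door sets Ready on every BP_button1 sharing one of its actor tags, linking doors and buttons by tag.
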(event `self.ReceiveBeginPlay`
  (add `PaperFlipbookComponent.OnFinishedPlaying` (`self.RenderComponent`) (delegate `FlipbookFinishEvent`)))

(event `FlipbookFinishEvent`
  (for _array_element (`self.Tags`)
    (bind _outactors (`GameplayStatics.GetAllActorsOfClassWithTag` "/Game/Assets/puzzle_platformer_kit/BP/BP_button1.BP_button1_C" _array_element))
    (for _array_element_2 _outactors
      (set `/Game/Assets/puzzle_platformer_kit/BP/BP_button1.Ready` true _array_element_2))))

(event `Trigger`
  (bind _rendercomponent (`self.RenderComponent`))
  (if (`PaperFlipbookComponent.IsPlaying` _rendercomponent)
    (set `self.doorOn` (not (`self.doorOn`)))
    (`PaperFlipbookComponent.Reverse` _rendercomponent)
    (elif (`self.doorOn`)
      (set `self.doorOn` false)
      (`PaperFlipbookComponent.ReverseFromEnd` _rendercomponent)
      (else
        (set `self.doorOn` true)
        (`PaperFlipbookComponent.Play` _rendercomponent)))))

(fn `UserConstructionScript`
  (bind _rendercomponent (`self.RenderComponent`))
  (`PaperFlipbookComponent.Stop` _rendercomponent)
  (`PaperFlipbookComponent.SetPlaybackPosition` _rendercomponent 0.0 false)
  (`PaperFlipbookComponent.SetLooping` _rendercomponent false))