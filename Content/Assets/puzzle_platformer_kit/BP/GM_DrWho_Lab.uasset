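; Game mode for the DrWho Lab level that respawns the player character after death.
; Every tick, and on RespawnRefresh, it checks whether the player's Pawn_DrWho_Lab is dead.
; If so, it waits briefly, spawns a new pawn at the checkpoint RespawnTransform, possesses it and calls RespawnRefresh again.
; The Respawn and NewFunction functions are empty stubs.
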(event `RespawnRefresh`
  ;[1 1 1] Checkpoint
  (bind _aspaper_character (cast `PaperCharacter` (`GameplayStatics.GetPlayerCharacter` 0) :!label _label))
  (bind _aspawn_dr_who_lab (cast `/Game/Assets/puzzle_platformer_kit/BP/Pawn_DrWho_Lab` _aspaper_character))
  (if (`/Game/Assets/puzzle_platformer_kit/BP/Pawn_DrWho_Lab.isDead` _aspawn_dr_who_lab)
    (`KismetSystemLibrary.Delay` 2.0) ; Wait 2 seconds before respawn
    (bind _returnvalue (`|SpawnActorFromClass` "/Game/Assets/puzzle_platformer_kit/BP/Pawn_DrWho_Lab.Pawn_DrWho_Lab_C" (`self.respawnTransform`) "Undefined" "OverrideRootScale" null null)) ; Respawn player
    (`Controller.Possess` (`GameplayStatics.GetPlayerController` 0) _returnvalue) ; Posess player
    (`self.RespawnRefresh`) ; Allow new player to use the checkpoint system
  ))

(event `self.ReceiveTick`
  (params (DeltaSeconds :type "Float (single-precision)"))
  ;[1 1 1] Checkpoint
  (goto _label))

(fn `New Function`)

(fn `Respawn`)

(fn `UserConstructionScript`)