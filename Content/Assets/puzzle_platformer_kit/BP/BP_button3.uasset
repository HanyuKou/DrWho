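; BP_button3 is a one-shot sprite button for a puzzle platformer, pressed when the player pawn or a cube overlaps its box.
; Pressing it clears ButtonOn, swaps the sprite and checks each of its tags.
; Buttons sharing a tag act as an AND group, calling TriggerConnected only once none is still on.
; TempTrigger offers a second press path with a different sprite and the same group check.
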(event `self.ReceiveBeginPlay`
  (`parent.ReceiveBeginPlay`))

(event `self.BoxOverlapEvent`
  (bind _box (`self.Box`))
  (if (not (== (+ (`KismetArrayLibrary.Array_Length` (`PrimitiveComponent.GetOverlappingActors` _box "/Game/Assets/puzzle_platformer_kit/BP/Pawn_DrWho_Lab.Pawn_DrWho_Lab_C")) (`KismetArrayLibrary.Array_Length` (`PrimitiveComponent.GetOverlappingActors` _box "/Game/Assets/puzzle_platformer_kit/BP/BP_cube.BP_cube_C"))) 0))
    (`/Engine/EditorBlueprintResources/StandardMacros.DoOnce` false
      (:`Completed`
        (set `self.ButtonOn` false)
        (`PaperSpriteComponent.SetSprite` (`self.RenderComponent`) "/Game/Assets/puzzle_platformer_kit/Sprite/button3_2.button3_2")
        (for _array_element (`self.Tags`) :!label _label
          (set `self.checkResult` true)
          (bind _outactors (`GameplayStatics.GetAllActorsOfClassWithTag` "BP_button3_C" _array_element))
          (if (== (`KismetArrayLibrary.Array_Length` _outactors) 1)
            (`self.TriggerConnected` false :!label _label_2)
            (else
              (for _array_element_2 _outactors
                (if (`/Game/Assets/puzzle_platformer_kit/BP/BP_button1.ButtonOn` _array_element_2)
                  (set `self.checkResult` false)
                  (break)))
              (if (`self.checkResult`)
                (goto _label_2)))))))))

(event `self.tempTrigger`
  (if (`self.ButtonOn`)
    (set `self.ButtonOn` false)
    (`PaperSpriteComponent.SetSprite` (`self.RenderComponent`) "/Game/Assets/puzzle_platformer_kit/Sprite/button1_2.button1_2")
    (goto _label)))

(fn `UserConstructionScript`
  (`parent.UserConstructionScript`))