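; EndGoal_BP is a level-end goal trigger that fires once when anything begins overlapping its Box.
; It sets JumpToLevelSelectMenu on Dr_Who_Game_Instance, finds the current level among LevelListDataTable row names and stores the following row as NextLevel, without a bounds check.
; It then opens LoadingLevel, which also happens if the game instance cast fails.
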(event `self.Box.OnComponentBeginOverlap`
  (params (OverlappedComponent :type "PrimitiveComponent Object Reference") (OtherActor :type "Actor Object Reference") (OtherComp :type "PrimitiveComponent Object Reference") (OtherBodyIndex :type Integer) (bFromSweep :type Boolean) (SweepResult :type "HitResult Structure (by ref)"))
  (`/Engine/EditorBlueprintResources/StandardMacros.DoOnce` false
    (:`Completed`
      (bind _asdr_who_game_instance (cast `/Game/Dr_Who_Game_Instance` (`GameplayStatics.GetGameInstance`))
        (:`then`
          (set `/Game/Dr_Who_Game_Instance.JumpToLevelSelectMenu` true _asdr_who_game_instance)
          (bind _returnvalue (`GameplayStatics.GetCurrentLevelName` true))
          (bind _outrownames (`DataTableFunctionLibrary.GetDataTableRowNames` "/Game/levelListDataTable.levelListDataTable"))
          (for (_array_element _array_index) _outrownames
            (if (== _array_element _returnvalue)
              (set `/Game/Dr_Who_Game_Instance.nextLevel` (`|GetArrayItem` _outrownames (+ _array_index 1)) _asdr_who_game_instance)
              (break))))
        (:`CastFailed`
          _))
      (`GameplayStatics.OpenLevelBySoftObjectPtr` "/Game/UI/loadingLevel.loadingLevel"))))

(fn `UserConstructionScript`)