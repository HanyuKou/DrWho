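; An interactable electric puzzle element that turns off lasers when the player has charged the lightning.
; On interact, it casts the player character to Pawn_DrWho and proceeds only if IsCharged is true.
; It treats each of its own Tags as a link, calling Trigger on every BP_laser1 actor that carries the same tag.
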(event `self.OnInteract`
  ;[1 1 1] Check if the player has charged the lighting
  (bind _aspawn_dr_who (cast `/Game/Character/Pawn_DrWho` (`GameplayStatics.GetPlayerCharacter` 0)))
  (if (`/Game/Character/Pawn_DrWho.isCharged` _aspawn_dr_who)
    ;[1 1 1] Turn off lazers
    (for _array_element (`self.Tags`)
      (bind _outactors (`GameplayStatics.GetAllActorsOfClassWithTag` "/Game/Assets/puzzle_platformer_kit/BP/BP_laser1.BP_laser1_C" _array_element))
      (for _array_element_2 _outactors
        (`/Game/Assets/puzzle_platformer_kit/BP/BP_laser1.Trigger` _array_element_2)))))

(fn `UserConstructionScript`
  (`parent.UserConstructionScript`))