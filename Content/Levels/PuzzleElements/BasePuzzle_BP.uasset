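; Base puzzle element that lets the player trigger an interaction while standing inside its Box volume.
; Overlap by Pawn_DrWho enables player 0 input and opens a Gate; any Pawn leaving disables input and closes it.
; Interact presses passing the Gate call OnInteract, which here only prints a test string.
; CanInteract always returns true and is not called in this graph.
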(event `OnInteract`
  (`KismetSystemLibrary.PrintString` "Base Interact Test"))

(event `InputAction|Interact`
  (params (Key :type "Key Structure"))
  ;[1 1 1] Player input check: Check if the player is close enough to interact
  (:`Pressed`
    (`/Engine/EditorBlueprintResources/StandardMacros.Gate` true :!label _label
      (:`Exit`
        (`self.OnInteract`)))))

(event `self.Box.OnComponentBeginOverlap`
  (params (OverlappedComponent :type "PrimitiveComponent Object Reference") (OtherActor :type "Actor Object Reference") (OtherComp :type "PrimitiveComponent Object Reference") (OtherBodyIndex :type Integer) (bFromSweep :type Boolean) (SweepResult :type "HitResult Structure (by ref)"))
  ;[1 1 1] Player input check: Check if the player is close enough to interact
  (cast `/Game/Character/Pawn_DrWho` OtherActor)
  (`self.EnableInput` (`GameplayStatics.GetPlayerController` 0))
  (goto _label :!via `Open`))

(event `self.Box.OnComponentEndOverlap`
  (params (OverlappedComponent :type "PrimitiveComponent Object Reference") (OtherActor :type "Actor Object Reference") (OtherComp :type "PrimitiveComponent Object Reference") (OtherBodyIndex :type Integer))
  ;[1 1 1] Player input check: Check if the player is close enough to interact
  (cast `Pawn` OtherActor)
  (`self.DisableInput` (`GameplayStatics.GetPlayerController` 0))
  (goto _label :!via `Close`))

(fn `canInteract`
  (params (Player :type "/Game/Character/Pawn_DrWho Object Reference"))
  (returns (CanInteract :type Boolean))
  (return true))

(fn `UserConstructionScript`)