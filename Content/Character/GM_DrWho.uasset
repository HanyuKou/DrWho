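; GM_DrWho, apparently a game mode, handles checkpoint respawning for the Pawn_DrWho player character.
; Tick and the RespawnRefresh event share one chain that casts the player character and checks IsDead.
; On death it delays briefly, spawns a GM_DrWho_Lab actor at RespawnTransform, calls Possess on the player controller, then calls RespawnRefresh again.
; The Respawn and New Function graphs are empty.
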(event `RespawnRefresh`
  ;[1 1 1] Checkpoint
  (bind _aspaper_character (cast `PaperCharacter` (`GameplayStatics.GetPlayerCharacter` 0) :!label _label))
  (bind _aspawn_dr_who (cast `/Game/Character/Pawn_DrWho` _aspaper_character))
  (if (`/Game/Character/Pawn_DrWho.IsDead` _aspawn_dr_who)
    (`KismetSystemLibrary.Delay` 1.5) ; Wait 2 seconds before respawn
    (`|SpawnActorFromClass` "/Game/Assets/puzzle_platformer_kit/BP/GM_DrWho_Lab.GM_DrWho_Lab_C" (`self.respawnTransform`) "Undefined" "MultiplyWithRoot" null null) ; Respawn player
    (`Controller.Possess` (`GameplayStatics.GetPlayerController` 0) null) ; Posess player
    (`self.RespawnRefresh`) ; Allow new player to use the checkpoint system
  ))

(event `self.ReceiveTick`
  (params (DeltaSeconds :type "Float (single-precision)"))
  ;[1 1 1] Checkpoint
  (goto _label))

(fn `New Function`)

(fn `Respawn`)

(fn `UserConstructionScript`)