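; Game mode for the Doctor Who character that respawns the player when their character is destroyed.
; On BeginPlay it binds to the player Paper character's OnDestroyed event.
; When that fires, it waits briefly, spawns a new Character_DrWho at RespawnTransform, which serves as the checkpoint, and possesses it with the player controller.
; It then calls Respawn to rebind the destroy event, so the cycle repeats for each new character.
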(event `Respawn`
  ;[1 1 1] Checkpoint
  (bind _aspaper_character (cast `PaperCharacter` (`GameplayStatics.GetPlayerCharacter` 0) :!label _label))
  (add `self.OnDestroyed` _aspaper_character (delegate `OnRespawnCall`)) ; On Player destory, call OnRespawnCall
)

(event `self.ReceiveBeginPlay`
  ;[1 1 1] Checkpoint
  (goto _label))

(event `OnRespawnCall` :!signature `self.OnDestroyed`
  (params (DestroyedActor :type "Actor Object Reference"))
  ;[1 1 1] Checkpoint
  (`KismetSystemLibrary.Delay` 2.0) ; Wait 2 seconds before respawn
  (bind _returnvalue (`|SpawnActorFromClass` "/Game/DoctorWhoCharacter/Character_DrWho.Character_DrWho_C" (`self.respawnTransform`) "Undefined" "MultiplyWithRoot" null null)) ; Respawn player
  (`Controller.Possess` (`GameplayStatics.GetPlayerController` 0) _returnvalue) ; Posess player
  (`self.Respawn`) ; Call Respawn Event
)

(fn `UserConstructionScript`)